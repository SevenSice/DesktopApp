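; BP_FunctionLibrary is a Blueprint function library with small debug and input helper functions.
; GetTime prints the hours, minutes, seconds and frames of the current timecode as separate on-screen strings through a Sequence.
; MouseHitResult returns the hit result of a complex Visibility-channel trace under the first player controller's cursor.
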(fn GetTime
  (bind _returnvalue (Class|TimeManagementBlueprintLibrary|GetTimecode))
  (bind (_hours _minutes _seconds _frames) (Utilities|Struct|BreakTimecode _returnvalue))
  (Utilities|FlowControl|Sequence
    (:then_1
      (Development|PrintString 0 (Utilities|String|ToString(Integer) _hours)))
    (:then_2
      (Development|PrintString 0 (Utilities|String|ToString(Integer) _minutes)))
    (:then_3
      (Development|PrintString 0 (Utilities|String|ToString(Integer) _seconds)))
    (:then_4
      (Development|PrintString 0 (Utilities|String|ToString(Integer) _frames)))))

(fn MouseHitResult
  (return (.HitResult (Game|Player|GetHitResultUnderCursorbyChannel (Game|GetPlayerController 0) "TraceTypeQuery1" true))))