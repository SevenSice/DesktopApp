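; Construction-script spline tool that scatters copies of a static mesh along a spline, apparently for placing vegetation.
; It spaces NumberOfMeshes components evenly from start to end of Spline1 at a uniform default scale.
; OrientToSpline rotates each mesh to follow the spline; otherwise optional flags randomize per-axis scale within a min/max range and yaw.
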(fn ConstructionScript
  (bind _number_of_meshes (Variables|Default|GetNumber%20of%20meshes))
  (bind _randomminsize (Variables|Default|GetRandomMinSize))
  (bind _randommaxsize (Variables|Default|GetRandomMaxSize))
  (bind _returnvalue (Math|Random|RandomFloatinRange _randomminsize _randommaxsize))
  (bind _returnvalue_2 (- _number_of_meshes 1))
  (if (> _number_of_meshes 0)
    (for _index (range 0 _returnvalue_2) ; Repeat loop for each mesh to add
      (bind _returnvalue_3 (AddComponent|AddStaticMeshComponent false (Math|Transform|MakeTransform (Math|Transform|InverseTransformLocation (Transformation|GetActorTransform) (Spline|GetLocationatDistanceAlongSpline (Variables|Default|GetSpline1) (* _index (/ (Spline|GetSplineLength (Variables|Default|GetSpline1)) (Math|Conversions|ToFloat(Integer) _returnvalue_2))) "World")) "0, 0, 0" "0.600000,0.600000,0.600000"))) ; Add static mesh component
      (if (Variables|Default|GetOrient%20to%20spline)
        (Transformation|SetWorldRotation _returnvalue_3 (Spline|GetRotationatDistanceAlongSpline (Variables|Default|GetSpline1) (* _index (/ (Spline|GetSplineLength (Variables|Default|GetSpline1)) (Math|Conversions|ToFloat(Integer) _returnvalue_2))) "World") false false) ; Rotate mesh to match direction of spline at its position
        (else
          (Utilities|FlowControl|Sequence
            (:then_0
              (if (Variables|Default|GetRandomSize)
                (Transformation|SetWorldScale3D _returnvalue_3 (Math|Vector|MakeVector _returnvalue _returnvalue _returnvalue))))
            (:then_1
              (if (Variables|Default|GetRandomDirection)
                (Transformation|SetWorldRotation _returnvalue_3 (Math|Rotator|MakeRotator (.roll (Transformation|GetWorldRotation _returnvalue_3)) (.pitch (Transformation|GetWorldRotation _returnvalue_3)) (Math|Random|RandomFloatinRange -1.8e+02 1.8e+02)) false false) ; Rotate mesh to match direction of spline at its position
              ))))))))