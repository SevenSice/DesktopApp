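; Player pawn with click-to-move navigation that changes with its move state: Observer, In Sky or On Landed.
; A mouseClick helper separates single from double clicks.
; In Observer, single-clicking a BP_TargetPoint moves to its transform, enters In Sky and sets the spring arm length.
; Double-clicks project the cursor hit onto the navmesh, then move directly when In Sky or via SimpleMoveToLocation when On Landed.
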(event EventTick
  (params (DeltaSeconds :type Float%20%28single-precision%29)))

(event EventBeginPlay
  (Variables|Default|SetMove_State "Observer"))

(event Input|ActionEvents|InputActionClick
  (params (Key :type Key%20Structure))
  (bind _mousehitresult (CallFunction|MouseHitResult "TraceTypeQuery1"))
  (bind _returnvalue (Class|NavigationSystemV1|GetNavigationSystem))
  (bind _mousehitresult_2 (CallFunction|MouseHitResult "TraceTypeQuery1"))
  (bind _returnvalue_2 (Class|NavigationSystemV1|GetNavigationSystem))
  (bind _location (Collision|BreakHitResult _mousehitresult))
  (bind _location_2 (Collision|BreakHitResult _mousehitresult_2))
  (bind _projectedlocation (AI|Navigation|ProjectPointtoNavigation _returnvalue _location 0 "/Script/NavigationSystem.NavigationQueryFilter" (Math|Vector|MakeVector 5e+02 5e+02 5e+02)))
  (bind _projectedlocation_2 (AI|Navigation|ProjectPointtoNavigation _returnvalue_2 _location_2 0 "/Script/NavigationSystem.NavigationQueryFilter" (Math|Vector|MakeVector 5e+02 5e+02 5e+02)))
  (:Pressed
    (Utilities|MouseClick 0.35 1e+01 :!label _label
      (:SingleClick
        (switch Utilities|FlowControl|Switch|SwitchonMotionState (Variables|Default|GetMove_State)
          (:Observer
            (bind _asbp_target_point (Utilities|Casting|CastToBP_TargetPoint (.HitActor (Collision|BreakHitResult (CallFunction|MouseHitResult "TraceTypeQuery1")))))
            (Class|MCharacter|MoveStarttoLocationandRotation (Default|GetPonitLocation _asbp_target_point) (Default|GetPointRotation _asbp_target_point))
            (CallFunction|SetInitinSky))))
      (:DoubleClick
        (switch Utilities|FlowControl|Switch|SwitchonMotionState (Variables|Default|GetMove_State)
          (:InSky
            (if (not (Math|Vector|Equal(Vector) _projectedlocation_2 (Transformation|GetWorldLocation (Variables|Default|GetCameraComp)) 5.0))
              (Class|MCharacter|MoveStarttoLocationandRotation (+ _projectedlocation_2 (Math|Vector|MakeVector 0.0 0.0 (Variables|/Script/Engine.CapsuleComponent|GetCapsuleHalfHeight (Variables|Default|GetCapsuleComponent)))) (Transformation|GetActorRotation))))
          (:OnLanded
            (if (not (Math|Vector|Equal(Vector) _projectedlocation (Transformation|GetWorldLocation (Variables|Default|GetCameraComp)) 5.0))
              (AI|Navigation|SimpleMovetoLocation (Pawn|GetController) (+ _projectedlocation (Math|Vector|MakeVector 0.0 0.0 (Variables|/Script/Engine.CapsuleComponent|GetCapsuleHalfHeight (Variables|Default|GetCapsuleComponent)))))))))))
  (:Released
    (goto _label ClickUp)))

(fn ConstructionScript)

(fn SetInitinSky
  (Variables|Default|SetMove_State "InSky")
  (Variables|/Script/Engine.SpringArmComponent|SetTargetArmLength (Variables|Default|GetSpringArmComp) 3e+01))