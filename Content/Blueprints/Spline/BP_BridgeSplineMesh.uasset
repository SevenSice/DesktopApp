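; Construction-script Blueprint that lays a mesh along a spline, apparently to build a bridge.
; It samples Spline at even distances, with the segment count derived from spline length over a clamped MeshLength, and rebuilds a second spline, Point, from those samples.
; Each Point segment gets a spline mesh component using its locations and tangents.
; Samples are read in world space but written to Point as local.
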(event EventBeginPlay)

(event Collision|EventActorBeginOverlap
  (params (OtherActor :type Actor%20Object%20Reference)))

(event EventTick
  (params (DeltaSeconds :type Float%20%28single-precision%29)))

(fn ConstructionScript
  (bind _pointarray (Variables|Default|GetPointArray))
  (bind _spline (Variables|Default|GetSpline))
  (bind _meshlength (Variables|Default|GetMeshLength))
  (bind _point (Variables|Default|GetPoint))
  (bind _returnvalue (Spline|GetSplineLength _spline))
  (bind _returnvalue_2 (Math|Float|Clamp(Float) _meshlength 1e+01 1e+04))
  (bind _returnvalue_3 (/ _returnvalue _returnvalue_2))
  (bind _returnvalue_4 (Math|Float|Truncate _returnvalue_3))
  (for _index (range 0 _returnvalue_4) ; Repeat loop for each mesh to add
    (Utilities|Array|Add (Variables|Default|GetPointArray) (Spline|GetLocationatDistanceAlongSpline (Variables|Default|GetSpline) (* _index (/ (Spline|GetSplineLength (Variables|Default|GetSpline)) (Math|Conversions|ToFloat(Integer) _returnvalue_4))) "World")))
  (Spline|SetSplinePoints (Variables|Default|GetPoint) _pointarray "Local" true)
  (for _index_2 (range 0 (- (Utilities|Array|Length _pointarray) 2)) ; 循环
    ;[1 1 1] Set Mesh
    (bind _returnvalue_5 (AddComponent|AddSplineMeshComponent true))
    (Components|StaticMesh|SetStaticMesh _returnvalue_5 (Variables|Default|GetMesh))
    (Transformation|AttachComponentToComponent _returnvalue_5 (Variables|Default|GetDefaultSceneRoot) "None" "KeepWorld" "KeepWorld" "KeepWorld" true)
    (SplineMesh|SetStartandEnd _returnvalue_5 (.Location (Spline|GetLocationandTangentatSplinePoint _point _index_2 "Local")) (.Tangent (Spline|GetLocationandTangentatSplinePoint _point _index_2 "Local")) (.Location (Spline|GetLocationandTangentatSplinePoint _point (+ _index_2 1) "Local")) (.Tangent (Spline|GetLocationandTangentatSplinePoint _point (+ _index_2 1) "Local")) true :!class /Script/Engine.SplineMeshComponent) ; 设置起点和终点
  ))